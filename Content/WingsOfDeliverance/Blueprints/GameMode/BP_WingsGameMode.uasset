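; Game mode Blueprint for Wings of Deliverance that controls input mode and pausing for the first local player.
; On BeginPlay it sets game-only input.
; PauseGame pauses the game, switches to UI-only input and shows the mouse cursor.
; UnpauseGame reverses this by resuming play, restoring game-only input and hiding the cursor.
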(event EventBeginPlay
  (Input|SetInputModeGameOnly (Game|GetPlayerController 0) false))

(fn ConstructionScript)

(fn PauseGame
  (bind _returnvalue (Game|GetPlayerController 0))
  (Game|SetGamePaused true)
  (Input|SetInputModeUIOnly _returnvalue 0 "DoNotLock" false)
  (Variables|/Script/Engine.PlayerController|SetbShowMouseCursor _returnvalue true))

(fn UnpauseGame
  (bind _returnvalue (Game|GetPlayerController 0))
  (Game|SetGamePaused false)
  (Input|SetInputModeGameOnly _returnvalue false)
  (Variables|/Script/Engine.PlayerController|SetbShowMouseCursor _returnvalue false))