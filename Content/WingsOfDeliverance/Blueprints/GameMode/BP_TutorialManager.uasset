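; Tutorial manager for Wings of Deliverance that pauses the game to show a sequence of tutorial widgets and gates player input.
; It shows the first widget and disables input shortly after BeginPlay, then four one-shot trigger overlaps pause and show the later prompts, most re-enabling input.
; Jump dismisses the second prompt, unpauses and disables input again; other prompts are not dismissed here.
; An unconnected chain holds an unused wing-flap impulse, stamina and sound sequence.
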(event OnComponentBeginOverlap(Trigger1)
  (params (OverlappedComponent :type Primitive%20Component%20Object%20Reference) (OtherActor :type Actor%20Object%20Reference) (OtherComp :type Primitive%20Component%20Object%20Reference) (OtherBodyIndex :type Integer) (bFromSweep :type Boolean) (SweepResult :type Hit%20Result%20Structure%20%28by%20ref%29))
  (bind _returnvalue (Game|GetPlayerController 0))
  (if (not (Variables|Default|GetEvent1))
    (bind _asbp_wings_character (Utilities|Casting|CastToBP_WingsCharacter OtherActor))
    (Variables|Default|SetEvent1 true)
    (Input|EnableInput _asbp_wings_character _returnvalue)
    (bind _returnvalue_2 (UserInterface|CreateWidget "/Game/WingsOfDeliverance/UI/WBP_Tutorial2.WBP_Tutorial2_C"))
    (UserInterface|Viewport|AddtoPlayerScreen _returnvalue_2)
    (bind _asbp_wings_game_mode (Utilities|Casting|CastToBP_WingsGameMode (Game|GetGameMode)))
    (Default|PauseGame _asbp_wings_game_mode)
    (Input|SetInputModeGameandUI _returnvalue 0 "DoNotLock" true false)))

(event OnComponentBeginOverlap(Trigger2)
  (params (OverlappedComponent :type Primitive%20Component%20Object%20Reference) (OtherActor :type Actor%20Object%20Reference) (OtherComp :type Primitive%20Component%20Object%20Reference) (OtherBodyIndex :type Integer) (bFromSweep :type Boolean) (SweepResult :type Hit%20Result%20Structure%20%28by%20ref%29))
  (if (not (Variables|Default|GetEvent2))
    (Utilities|Casting|CastToBP_WingsCharacter OtherActor)
    (bind _asbp_wings_game_mode (Utilities|Casting|CastToBP_WingsGameMode (Game|GetGameMode)))
    (Default|PauseGame _asbp_wings_game_mode)
    (bind _returnvalue (UserInterface|CreateWidget "/Game/WingsOfDeliverance/UI/WBP_Tutorial3.WBP_Tutorial3_C"))
    (UserInterface|Viewport|AddtoPlayerScreen _returnvalue)
    (Variables|Default|SetEvent2 true)))

(event OnComponentBeginOverlap(Trigger3)
  (params (OverlappedComponent :type Primitive%20Component%20Object%20Reference) (OtherActor :type Actor%20Object%20Reference) (OtherComp :type Primitive%20Component%20Object%20Reference) (OtherBodyIndex :type Integer) (bFromSweep :type Boolean) (SweepResult :type Hit%20Result%20Structure%20%28by%20ref%29))
  (if (not (Variables|Default|GetEvent3))
    (bind _asbp_wings_character (Utilities|Casting|CastToBP_WingsCharacter OtherActor))
    (bind _asbp_wings_game_mode (Utilities|Casting|CastToBP_WingsGameMode (Game|GetGameMode)))
    (Default|PauseGame _asbp_wings_game_mode)
    (bind _returnvalue (UserInterface|CreateWidget "/Game/WingsOfDeliverance/UI/WBP_Tutorial4.WBP_Tutorial4_C"))
    (UserInterface|Viewport|AddtoPlayerScreen _returnvalue)
    (Input|EnableInput _asbp_wings_character (Game|GetPlayerController 0))
    (Variables|Default|SetEvent3 true)))

(event OnComponentBeginOverlap(Trigger4)
  (params (OverlappedComponent :type Primitive%20Component%20Object%20Reference) (OtherActor :type Actor%20Object%20Reference) (OtherComp :type Primitive%20Component%20Object%20Reference) (OtherBodyIndex :type Integer) (bFromSweep :type Boolean) (SweepResult :type Hit%20Result%20Structure%20%28by%20ref%29))
  (if (not (Variables|Default|GetEvent4))
    (bind _asbp_wings_character (Utilities|Casting|CastToBP_WingsCharacter OtherActor))
    (bind _asbp_wings_game_mode (Utilities|Casting|CastToBP_WingsGameMode (Game|GetGameMode)))
    (Default|PauseGame _asbp_wings_game_mode)
    (bind _returnvalue (UserInterface|CreateWidget "/Game/WingsOfDeliverance/UI/WBP_Tutorial5.WBP_Tutorial5_C"))
    (UserInterface|Viewport|AddtoPlayerScreen _returnvalue)
    (Input|EnableInput _asbp_wings_character (Game|GetPlayerController 0))
    (Variables|Default|SetEvent4 true)))

(event EventBeginPlay
  (Utilities|FlowControl|Delay 0.5)
  (bind _asbp_wings_game_mode (Utilities|Casting|CastToBP_WingsGameMode (Game|GetGameMode)))
  (Default|PauseGame _asbp_wings_game_mode)
  (bind _returnvalue (UserInterface|CreateWidget "/Game/WingsOfDeliverance/UI/WBP_Tutorial1.WBP_Tutorial1_C"))
  (UserInterface|Viewport|AddtoPlayerScreen _returnvalue)
  (bind _asbp_wings_character (Utilities|Casting|CastToBP_WingsCharacter (Game|GetPlayerCharacter 0)))
  (Input|DisableInput _asbp_wings_character (Game|GetPlayerController 0)))

(event Collision|EventActorBeginOverlap
  (params (OtherActor :type Actor%20Object%20Reference)))

(event EventTick
  (params (DeltaSeconds :type Float%20%28single-precision%29)))

(event Input|ActionEvents|InputActionJump
  (params (Key :type Key%20Structure :default "None"))
  (:Pressed
    (if (and (Variables|Default|GetEvent1) (not (Variables|Default|GetEvent1Complete)))
      (Variables|Default|SetEvent1Complete true)
      (bind _asbp_wings_character (Utilities|Casting|CastToBP_WingsCharacter (Game|GetPlayerCharacter 0)))
      (Widget|RemovefromParent (stale OnComponentBeginOverlap(Trigger1) _returnvalue_2))
      (bind _asbp_wings_game_mode (Utilities|Casting|CastToBP_WingsGameMode (Game|GetGameMode)))
      (Default|UnpauseGame _asbp_wings_game_mode)
      (Utilities|FlowControl|Delay 0.2)
      (Input|DisableInput _asbp_wings_character (Game|GetPlayerController 0)))))

(fn ConstructionScript)