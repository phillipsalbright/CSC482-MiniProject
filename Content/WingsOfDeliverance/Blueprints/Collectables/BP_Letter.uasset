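; BP_Letter is a collectable in Wings of Deliverance that ends the level when the player collects it.
; Its OnCollected event pauses the game, shows the WBP_LevelComplete widget and switches the player's controller to UI-only input with a visible cursor.
; It then hands its NextLevel value to the widget and plays a collection sound.
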(event EventBeginPlay)

(event Collision|EventActorBeginOverlap
  (params (OtherActor :type Actor%20Object%20Reference)))

(event EventTick
  (params (DeltaSeconds :type Float%20%28single-precision%29)))

(event EventOnCollected
  (params (Player :type BP%20Wings%20Character%20Object%20Reference))
  (Game|SetGamePaused true)
  (bind _returnvalue (UserInterface|CreateWidget "/Game/WingsOfDeliverance/UI/WBP_LevelComplete.WBP_LevelComplete_C"))
  (UserInterface|Viewport|AddtoPlayerScreen _returnvalue)
  (bind _asplayer_controller (Utilities|Casting|CastToPlayerController (Pawn|GetController Player)))
  (Input|SetInputModeUIOnly _asplayer_controller 0 "DoNotLock" false)
  (Variables|/Script/Engine.PlayerController|SetbShowMouseCursor _asplayer_controller true)
  (Default|SetNextLevel _returnvalue (Variables|Default|GetNextLevel))
  (Audio|PlaySound2D "/Game/WingsOfDeliverance/Audio/22-full_feather_collect_Cue.22-full_feather_collect_Cue" 1.0 1.0 0.0 0 0))

(fn ConstructionScript
  (|CallParentFunction))