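; BP_Sun_Square is a falling sun obstacle that drains the player's stamina.
; Tick moves the root straight down at FallSpeed, scaled by delta time.
; When a BP_WingsCharacter begins overlapping its Box, it calls RemoveStamina on that character with StaminaLoss.
; The construction script derives the root's scale from HeatIntensity, which sizes the whole obstacle.
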(event OnComponentBeginOverlap(Box)
  (params (OverlappedComponent :type Primitive%20Component%20Object%20Reference) (OtherActor :type Actor%20Object%20Reference) (OtherComp :type Primitive%20Component%20Object%20Reference) (OtherBodyIndex :type Integer) (bFromSweep :type Boolean) (SweepResult :type Hit%20Result%20Structure%20%28by%20ref%29))
  (bind _asbp_wings_character (Utilities|Casting|CastToBP_WingsCharacter OtherActor))
  (Default|RemoveStamina _asbp_wings_character (Variables|Default|GetstaminaLoss)))

(event EventTick
  (params (DeltaSeconds :type Float%20%28single-precision%29))
  (bind _defaultsceneroot (Variables|Default|GetDefaultSceneRoot))
  (bind _relativelocation (Variables|/Script/Engine.SceneComponent|GetRelativeLocation _defaultsceneroot))
  (Transformation|SetRelativeLocation _defaultsceneroot (Math|Vector|MakeVector (.x _relativelocation) (.y _relativelocation) (- (.z _relativelocation) (* DeltaSeconds (Variables|Default|GetfallSpeed)))) false false))

(fn ConstructionScript
  (Transformation|SetRelativeScale3D (Variables|Default|GetDefaultSceneRoot) (Math|Conversions|ToVector(Float) (Variables|Default|GetheatIntensity))))