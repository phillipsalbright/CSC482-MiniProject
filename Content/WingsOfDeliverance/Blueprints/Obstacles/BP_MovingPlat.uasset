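; BP_MovingPlat is a moving platform obstacle that shuttles back and forth along the world Y axis.
; Each Tick forces input into its FloatingPawnMovement component, using Direction scaled by delta seconds.
; A looping timer flips the sign of Direction every Dist seconds, so travel is bounded by time rather than position.
; BeginPlay also stores the mesh's start location, which nothing in these graphs reads.
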(event Custom|changeDir
  (Variables|Default|SetDirection (* (Variables|Default|GetDirection) -1.0)))

(event EventBeginPlay
  (Variables|Default|SetStartPos (Transformation|GetWorldLocation (Variables|Default|GetStaticMesh)))
  (Utilities|Time|SetTimerbyEvent (delegate Custom|changeDir) (Variables|Default|GetDist) true))

(event Collision|EventActorBeginOverlap
  (params (OtherActor :type Actor%20Object%20Reference)))

(event EventTick
  (params (DeltaSeconds :type Float%20%28single-precision%29))
  (Class|PawnMovementComponent|AddInputVector (Variables|Actor|GetFloatingPawnMovement) (Math|Vector|MakeVector 0.0 (* DeltaSeconds (Variables|Default|GetDirection)) 0.0) true))

(fn ConstructionScript)